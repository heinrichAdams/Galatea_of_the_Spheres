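; Player Blueprint that moves a physics-driven mesh from input axes and rotates a spring arm with the mouse.
; North-south input applies torque about the Arrow's right vector, scaled by a Torque variable, to roll the mesh.
; West-east input pushes it along that same vector with an inverted, fixed-scale force.
; Each tick adds mouse pitch and yaw to the spring arm's relative rotation, without delta-time scaling.
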(event EventTick
  (params (DeltaSeconds :type Float%20%28single-precision%29))
  ;[1 1 1] Mouse Controls
  (Transformation|AddRelativeRotation (Variables|Default|GetSpringArm) (Math|Rotator|MakeRotator 0.0 (Input|AxisValues|GetMousePitch) (Input|AxisValues|GetMouseYaw)) false false))

(event Input|AxisEvents|InputAxisSNMovement
  (params (AxisValue :type Float%20%28single-precision%29))
  ;[1 1 1] NS Movement
  (Class|PrimitiveComponent|AddTorqueinRadians (Variables|Default|GetPhysicalMesh) (* (Math|Vector|GetRightVector (Variables|Default|GetArrow)) (* AxisValue (Variables|Default|GetTorque))) "None" false))

(event Input|AxisEvents|InputAxisWEMovement
  (params (AxisValue :type Float%20%28single-precision%29))
  ;[1 1 1] WE Movement
  (Physics|AddForce (Variables|Default|GetPhysicalMesh) (* (Math|Vector|GetRightVector (Variables|Default|GetArrow)) (* (* AxisValue -1.0) 1e+04)) "None" false))

(fn ConstructionScript)