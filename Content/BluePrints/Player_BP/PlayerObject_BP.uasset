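; Player object that switches between a heavy dice cube and a light physics sphere on Space, with mouse-driven camera look.
; Each switch changes mesh, mass and damping, and velocity is reapplied when becoming a sphere.
; As a cube with near-zero vertical velocity, directional inputs drive per-direction timelines that lerp it along world axes through 90-degree flips, ending with a random sound.
; A shared LocationSet flag prevents recomputing endpoints mid-flip.
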(event Input|ActionEvents|InputActionLeft
  (params (Key :type Key%20Structure :default "None"))
  (bind _physicalmesh (Variables|Default|GetPhysicalMesh))
  (bind _physicalmesh_2 (Variables|Default|GetPhysicalMesh))
  (bind _returnvalue (Transformation|GetRelativeTransform _physicalmesh))
  ;[1 1 1] Object Movement
  (:Pressed
    (bind _returnvalue_2 (Class|PlayerObject|GetIsCube))
    (bind _returnvalue_3 (Physics|GetPhysicsLinearVelocity (Variables|Default|GetPhysicalMesh) "None"))
    (if (and _returnvalue_2 (Math|Vector|VectorIsNearlyZero (Math|Vector|MakeVector 0.0 0.0 (.z _returnvalue_3)) 1e+01))
      (if (Variables|Default|GetLocationSet)
        (bind _move (Timeline|Timeline_2 Play)
          (:Update
            (Transformation|SetWorldRotation _physicalmesh_2 (Math|Rotator|MakeRotator (.roll (Math|Rotator|Lerp(Rotator) (Variables|Default|GetStartRotation) (Variables|Default|GetEndRotation) _move)) 0.0 0.0) false true)
            (Transformation|SetWorldLocation _physicalmesh_2 (Math|Vector|Lerp(Vector) (Variables|Default|GetStartLocation) (Variables|Default|GetEndLocation) _move) false false)
            (Class|PrimitiveComponent|SetAllPhysicsAngularVelocityinRadians _physicalmesh_2 (Math|Vector|MakeVector 0.0 0.0 0.0) false))
          (:Finished
            (Variables|Default|SetLocationSet false)
            (Audio|PlaySoundatLocation (.OutItem (Utilities|Array|Random (Variables|Default|GetCube_Flip_Sounds))) (Math|Vector|Lerp(Vector) (Variables|Default|GetStartLocation) (Variables|Default|GetEndLocation) _move) "0, 0, 0" 1.0 1.0 -0.9 0 0 0)))
        (else
          (bind _output_get (Variables|Default|SetStartLocation (.location _returnvalue)))
          (Variables|Default|SetEndLocation (+ _output_get (Math|Vector|MakeVector 0.0 (* (Variables|Default|GetSpeed) (Class|PrimitiveComponent|GetMassScale (Variables|Default|GetPhysicalMesh) "None") -1.0) 0.0)))
          (bind _output_get_2 (Variables|Default|SetStartRotation (.rotation _returnvalue)))
          (Variables|Default|SetEndRotation (Math|Rotator|MakeRotator (+ (.roll _output_get_2) -9e+01) 0.0 0.0))
          (Variables|Default|SetLocationSet true)
          (Timeline|Timeline_2 PlayFromStart))))))

(event Input|ActionEvents|InputActionForward
  (params (Key :type Key%20Structure :default "None"))
  (bind _physicalmesh (Variables|Default|GetPhysicalMesh))
  (bind _physicalmesh_2 (Variables|Default|GetPhysicalMesh))
  (bind _returnvalue (Transformation|GetRelativeTransform _physicalmesh))
  ;[1 1 1] Object Movement
  (:Pressed
    (bind _returnvalue_2 (Class|PlayerObject|GetIsCube))
    (bind _returnvalue_3 (Physics|GetPhysicsLinearVelocity (Variables|Default|GetPhysicalMesh) "None"))
    (if (and _returnvalue_2 (Math|Vector|VectorIsNearlyZero (Math|Vector|MakeVector 0.0 0.0 (.z _returnvalue_3)) 1e+01))
      (if (Variables|Default|GetLocationSet)
        (bind _move (Timeline|Timeline_1 Play)
          (:Update
            (Transformation|SetWorldRotation _physicalmesh_2 (Math|Rotator|MakeRotator 0.0 (.pitch (Math|Rotator|Lerp(Rotator) (Variables|Default|GetStartRotation) (Variables|Default|GetEndRotation) _move)) 0.0) false true)
            (Transformation|SetWorldLocation _physicalmesh_2 (Math|Vector|Lerp(Vector) (Variables|Default|GetStartLocation) (Variables|Default|GetEndLocation) _move) false false)
            (Class|PrimitiveComponent|SetAllPhysicsAngularVelocityinRadians _physicalmesh_2 (Math|Vector|MakeVector 0.0 0.0 0.0) false))
          (:Finished
            (Variables|Default|SetLocationSet false)
            (Audio|PlaySoundatLocation (.OutItem (Utilities|Array|Random (Variables|Default|GetCube_Flip_Sounds))) (Math|Vector|Lerp(Vector) (Variables|Default|GetStartLocation) (Variables|Default|GetEndLocation) _move) "0, 0, 0" 1.0 1.0 -0.9 0 0 0)))
        (else
          (bind _output_get (Variables|Default|SetStartLocation (.location _returnvalue)))
          (Variables|Default|SetEndLocation (+ _output_get (Math|Vector|MakeVector (* (Variables|Default|GetSpeed) (Class|PrimitiveComponent|GetMassScale (Variables|Default|GetPhysicalMesh) "None") 1.0) 0.0 0.0)))
          (bind _output_get_2 (Variables|Default|SetStartRotation (.rotation _returnvalue)))
          (Variables|Default|SetEndRotation (Math|Rotator|MakeRotator 0.0 (+ (.pitch _output_get_2) -9e+01) 0.0))
          (Variables|Default|SetLocationSet true)
          (Timeline|Timeline_1 PlayFromStart))))))

(event Input|ActionEvents|InputActionRight
  (params (Key :type Key%20Structure :default "None"))
  (bind _physicalmesh (Variables|Default|GetPhysicalMesh))
  (bind _physicalmesh_2 (Variables|Default|GetPhysicalMesh))
  (bind _returnvalue (Transformation|GetRelativeTransform _physicalmesh))
  ;[1 1 1] Object Movement
  (:Pressed
    (bind _returnvalue_2 (Class|PlayerObject|GetIsCube))
    (bind _returnvalue_3 (Physics|GetPhysicsLinearVelocity (Variables|Default|GetPhysicalMesh) "None"))
    (if (and _returnvalue_2 (Math|Vector|VectorIsNearlyZero (Math|Vector|MakeVector 0.0 0.0 (.z _returnvalue_3)) 1e+01))
      (if (Variables|Default|GetLocationSet)
        (bind _move (Timeline|Timeline_0 Play)
          (:Update
            (Transformation|SetWorldRotation _physicalmesh_2 (Math|Rotator|MakeRotator (.roll (Math|Rotator|Lerp(Rotator) (Variables|Default|GetStartRotation) (Variables|Default|GetEndRotation) _move)) 0.0 0.0) false true)
            (Transformation|SetWorldLocation _physicalmesh_2 (Math|Vector|Lerp(Vector) (Variables|Default|GetStartLocation) (Variables|Default|GetEndLocation) _move) false false)
            (Class|PrimitiveComponent|SetAllPhysicsAngularVelocityinRadians _physicalmesh_2 (Math|Vector|MakeVector 0.0 0.0 0.0) false))
          (:Finished
            (Variables|Default|SetLocationSet false)
            (Audio|PlaySoundatLocation (.OutItem (Utilities|Array|Random (Variables|Default|GetCube_Flip_Sounds))) (Math|Vector|Lerp(Vector) (Variables|Default|GetStartLocation) (Variables|Default|GetEndLocation) _move) "0, 0, 0" 1.0 1.0 -0.9 0 0 0)))
        (else
          (bind _output_get (Variables|Default|SetStartLocation (.location _returnvalue)))
          (Variables|Default|SetEndLocation (+ _output_get (Math|Vector|MakeVector 0.0 (* (Variables|Default|GetSpeed) (Class|PrimitiveComponent|GetMassScale (Variables|Default|GetPhysicalMesh) "None") 1.0) 0.0)))
          (bind _output_get_2 (Variables|Default|SetStartRotation (.rotation _returnvalue)))
          (Variables|Default|SetEndRotation (Math|Rotator|MakeRotator (+ (.roll _output_get_2) 9e+01) 0.0 0.0))
          (Variables|Default|SetLocationSet true)
          (Timeline|Timeline_0 PlayFromStart))))))

(event Input|ActionEvents|InputActionBackward
  (params (Key :type Key%20Structure :default "None"))
  (bind _physicalmesh (Variables|Default|GetPhysicalMesh))
  (bind _physicalmesh_2 (Variables|Default|GetPhysicalMesh))
  (bind _returnvalue (Transformation|GetRelativeTransform _physicalmesh))
  ;[1 1 1] Object Movement
  (:Pressed
    (bind _returnvalue_2 (Class|PlayerObject|GetIsCube))
    (bind _returnvalue_3 (Physics|GetPhysicsLinearVelocity (Variables|Default|GetPhysicalMesh) "None"))
    (if (and _returnvalue_2 (Math|Vector|VectorIsNearlyZero (Math|Vector|MakeVector 0.0 0.0 (.z _returnvalue_3)) 1e+01))
      (if (Variables|Default|GetLocationSet)
        (bind _move (Timeline|MoveBackwardTimeline Play)
          (:Update
            (Transformation|SetWorldRotation _physicalmesh_2 (Math|Rotator|MakeRotator 0.0 (.pitch (Math|Rotator|Lerp(Rotator) (Variables|Default|GetStartRotation) (Variables|Default|GetEndRotation) _move)) 0.0) false true)
            (Transformation|SetWorldLocation _physicalmesh_2 (Math|Vector|Lerp(Vector) (Variables|Default|GetStartLocation) (Variables|Default|GetEndLocation) _move) false false)
            (Class|PrimitiveComponent|SetAllPhysicsAngularVelocityinRadians _physicalmesh_2 (Math|Vector|MakeVector 0.0 0.0 0.0) false))
          (:Finished
            (Variables|Default|SetLocationSet false)
            (Audio|PlaySoundatLocation (.OutItem (Utilities|Array|Random (Variables|Default|GetCube_Flip_Sounds))) (Math|Vector|Lerp(Vector) (Variables|Default|GetStartLocation) (Variables|Default|GetEndLocation) _move) "0, 0, 0" 1.0 1.0 -0.9 0 0 0)))
        (else
          (bind _output_get (Variables|Default|SetStartLocation (.location _returnvalue)))
          (Variables|Default|SetEndLocation (+ _output_get (Math|Vector|MakeVector (* (Variables|Default|GetSpeed) (Class|PrimitiveComponent|GetMassScale (Variables|Default|GetPhysicalMesh) "None") -1.0) 0.0 0.0)))
          (bind _output_get_2 (Variables|Default|SetStartRotation (.rotation _returnvalue)))
          (Variables|Default|SetEndRotation (Math|Rotator|MakeRotator 0.0 (+ (.pitch _output_get_2) 9e+01) 0.0))
          (Variables|Default|SetLocationSet true)
          (Timeline|MoveBackwardTimeline PlayFromStart))))))

(event Input|AxisEvents|InputAxisMousePitch
  (params (AxisValue :type Float%20%28single-precision%29))
  ;[1 1 1] Camera Control
  (Pawn|Input|AddControllerPitchInput (* AxisValue -1.0)))

(event Input|AxisEvents|InputAxisMouseYaw
  (params (AxisValue :type Float%20%28single-precision%29))
  ;[1 1 1] Camera Control
  (Pawn|Input|AddControllerYawInput AxisValue))

(event Input|KeyboardEvents|SpaceBar
  (params (Key :type Key%20Structure :default "None"))
  (bind _physicalmesh (Variables|Default|GetPhysicalMesh))
  (bind _physicalmesh_2 (Variables|Default|GetPhysicalMesh))
  (bind _physicalmesh_3 (Variables|Default|GetPhysicalMesh))
  ;[1 1 1] Object Movement
  (:Pressed
    (bind _returnvalue (Class|PlayerObject|GetIsCube))
    (Class|PlayerObject|SetIsCube (not _returnvalue))
    (if (Variables|Default|GetIsCube)
      (Components|StaticMesh|SetStaticMesh _physicalmesh "/Game/BluePrints/Player_BP/Dice.Dice")
      (Class|PrimitiveComponent|SetMassOverrideinKg _physicalmesh_3 "None" 9e+03 true)
      (Class|PrimitiveComponent|SetAngularDamping _physicalmesh_3 1.0)
      (Class|PrimitiveComponent|SetLinearDamping _physicalmesh_3 0.01)
      (else
        (bind _returnvalue_2 (Physics|GetPhysicsLinearVelocity _physicalmesh "None"))
        (Class|PlayerObject|SetVelocity _returnvalue_2)
        (Components|StaticMesh|SetStaticMesh _physicalmesh (Variables|Default|GetSphere))
        (Class|PrimitiveComponent|SetMassOverrideinKg _physicalmesh_2 "None" 5.0 true)
        (Class|PrimitiveComponent|SetAngularDamping _physicalmesh_2 -0.5)
        (Class|PrimitiveComponent|SetLinearDamping _physicalmesh_2 0.0)
        (Physics|SetPhysicsLinearVelocity _physicalmesh_2 (Variables|Default|GetVelocity) false "None")))))

(fn ConstructionScript)