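; Responsive pillar Blueprint that moves its IceCream component vertically according to the mass of the player's PhysicalMesh.
; Collider overlap events toggle a Move flag, and while it is set Tick raises the component for a light player and lowers it otherwise.
; The per-tick offset adds DeltaSeconds to the signed Speed instead of multiplying them.
; BeginPlay computes height limits, both above the start position, but movement never checks them.
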(event OnComponentBeginOverlap(Collider)
  (params (OverlappedComponent :type Primitive%20Component%20Object%20Reference) (OtherActor :type Actor%20Object%20Reference) (OtherComp :type Primitive%20Component%20Object%20Reference) (OtherBodyIndex :type Integer) (bFromSweep :type Boolean) (SweepResult :type Hit%20Result%20Structure%20%28by%20ref%29))
  (Variables|Default|SetMove true))

(event OnComponentEndOverlap(Collider)
  (params (OverlappedComponent :type Primitive%20Component%20Object%20Reference) (OtherActor :type Actor%20Object%20Reference) (OtherComp :type Primitive%20Component%20Object%20Reference) (OtherBodyIndex :type Integer))
  (Variables|Default|SetMove false))

(event EventBeginPlay
  ;[1 1 1] Initialization
  (bind _output_get (Variables|Default|SetDefaultPosition (Transformation|GetWorldLocation (Variables|Default|GetIceCream))))
  (Variables|Default|SetMaxHeight (+ _output_get "0, 0,100.000000"))
  (Variables|Default|SetMinHeight (- _output_get "0, 0,-100.000000")))

(event EventTick
  (params (DeltaSeconds :type Float%20%28single-precision%29))
  (bind _icecream (Variables|Default|GetIceCream))
  (if (Variables|Default|GetMove)
    (bind _asplayer_bp (Utilities|Casting|CastToPlayer_BP (Game|Player|GetPlayerPawn 0)))
    (if (< (Physics|GetMass (Variables|/Game/BluePrints/Player_BP/Player_BP.Player_BP_C|GetPhysicalMesh _asplayer_bp)) 5e+01)
      (if true
        (Transformation|AddLocalOffset _icecream (Math|Vector|MakeVector 0.0 0.0 (+ DeltaSeconds (Variables|Default|GetSpeed))) false false))
      (else
        (Transformation|AddLocalOffset _icecream (Math|Vector|MakeVector 0.0 0.0 (+ DeltaSeconds (* (Variables|Default|GetSpeed) -1.0))) false false)))))

(fn ConstructionScript)