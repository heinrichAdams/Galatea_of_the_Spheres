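; Checkpoint actor that sets the player's respawn point when touched.
; On Box overlap by a Player_BP, it writes the Scene component's world location, with zero rotation and unit scale, into the player's RespawnLocation.
; It then swaps a skeletal mesh material slot to M_Checked as visual confirmation.
; Leftover debug and objective-check nodes are disconnected and never run.
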(event OnComponentBeginOverlap(Box)
  (params (OverlappedComponent :type Primitive%20Component%20Object%20Reference) (OtherActor :type Actor%20Object%20Reference) (OtherComp :type Primitive%20Component%20Object%20Reference) (OtherBodyIndex :type Integer) (bFromSweep :type Boolean) (SweepResult :type Hit%20Result%20Structure%20%28by%20ref%29))
  (bind _asplayer_bp (Utilities|Casting|CastToPlayer_BP OtherActor))
  (Variables|/Game/BluePrints/Player_BP/Player_BP.Player_BP_C|SetRespawnLocation _asplayer_bp (Math|Transform|MakeTransform (.Location (Math|Transform|BreakTransform (Transformation|GetWorldTransform (Variables|Default|GetScene))))))
  (Rendering|Material|SetMaterial (Variables|Default|GetSkeletalMesh) 1 "/Game/BluePrints/Checkpoint_BP/Checkpoint_Flag/M_Checked.M_Checked"))

(event Collision|EventActorBeginOverlap
  (params (OtherActor :type Actor%20Object%20Reference))
  ;[1 1 1] Set Player Checkpoint
)

(fn ConstructionScript)