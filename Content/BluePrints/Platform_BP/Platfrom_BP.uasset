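; Moving platform Blueprint that shuttles its StaticMesh back and forth and sinks when hit by something too heavy.
; Two timelines, kept running from Tick via the EndOfTrack flag, restart each other and add scaled relative X offsets, despite their "Vertical_Track" names.
; A hit from a component with mass above MaxWeight lowers the mesh's Z by FallSpeed, then re-enters the same track logic.
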(event OnComponentHit(StaticMesh)
  (params (HitComponent :type Primitive%20Component%20Object%20Reference) (OtherActor :type Actor%20Object%20Reference) (OtherComp :type Primitive%20Component%20Object%20Reference) (NormalImpulse :type Vector :default "0, 0, 0") (Hit :type Hit%20Result%20Structure%20%28by%20ref%29))
  (bind _staticmesh (Variables|Default|GetStaticMesh))
  (bind _staticmesh_2 (Variables|Default|GetStaticMesh))
  (if (not (<= (Physics|GetMass OtherComp) (Variables|Default|GetMaxWeight)))
    (Transformation|SetRelativeLocation _staticmesh_2 (Math|Vector|MakeVector 0.0 0.0 (- (.z (Variables|/Script/Engine.SceneComponent|GetRelativeLocation _staticmesh_2)) (Variables|Default|GetFallSpeed))) false false)
    (if (Variables|Default|GetEndOfTrack)
      (bind _vertical_track (Timeline|Vertical_Track_Reverse Play)
        (:Update
          (Transformation|AddRelativeLocation _staticmesh (Math|Vector|MakeVector (* _vertical_track (* (Variables|Default|GetDistanceToTravel) -1.0)) 0.0 0.0) false false))
        (:Finished
          (Variables|Default|SetEndOfTrack false)
          (bind _vertical_track_2 (Timeline|Vertical_Track PlayFromStart)
            (:Update
              (Transformation|AddRelativeLocation _staticmesh (Math|Vector|MakeVector (* _vertical_track_2 (Variables|Default|GetDistanceToTravel)) 0.0 0.0) false false))
            (:Finished
              (Variables|Default|SetEndOfTrack true)
              (Timeline|Vertical_Track_Reverse PlayFromStart)))))
      (else
        (Timeline|Vertical_Track Play)))))

(event EventTick
  (params (DeltaSeconds :type Float%20%28single-precision%29))
  (bind _staticmesh (Variables|Default|GetStaticMesh))
  (if (Variables|Default|GetEndOfTrack)
    (bind _vertical_track (Timeline|Vertical_Track_Reverse Play)
      (:Update
        (Transformation|AddRelativeLocation _staticmesh (Math|Vector|MakeVector (* _vertical_track (* (Variables|Default|GetDistanceToTravel) -1.0)) 0.0 0.0) false false))
      (:Finished
        (Variables|Default|SetEndOfTrack false)
        (bind _vertical_track_2 (Timeline|Vertical_Track PlayFromStart)
          (:Update
            (Transformation|AddRelativeLocation _staticmesh (Math|Vector|MakeVector (* _vertical_track_2 (Variables|Default|GetDistanceToTravel)) 0.0 0.0) false false))
          (:Finished
            (Variables|Default|SetEndOfTrack true)
            (Timeline|Vertical_Track_Reverse PlayFromStart)))))
    (else
      (Timeline|Vertical_Track Play))))

(fn ConstructionScript)