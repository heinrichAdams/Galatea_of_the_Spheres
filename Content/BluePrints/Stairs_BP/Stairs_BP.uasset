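; Stairs actor that moves vertically back and forth in an endless loop from BeginPlay.
; A FlipFlop alternates Position_Timeline between forward and reverse on each finish, with the Reversed bool swapping the starting direction so blocks can alternate.
; Each update offsets the current location by a lerp between small up and down steps, so the timeline drives per-update movement rather than fixed endpoints.
; Tick runs a GetAllActorsOfClass whose result is unused.
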(event EventBeginPlay
  (bind _returnvalue (Transformation|GetActorLocation))
  (bind _reversed (Variables|Default|GetReversed))
  ;[1 1 1] Start, Repeat & Reverse
  (Utilities|FlowControl|FlipFlop :!label _label
    (:A
      (if _reversed ; Reverses Direction if bool
        (bind _position (Timeline|Position_Timeline ReverseFromEnd)
          (:Update
            ;[1 1 1] Movement
            (Transformation|SetActorLocation (Math|Vector|Lerp(Vector) (+ _returnvalue "0, 0,2.000000") (+ _returnvalue "0, 0,-2.000000") _position) false false))
          (:Finished
            (goto _label)))
        (else
          (Timeline|Position_Timeline PlayFromStart))))
    (:B
      (if _reversed
        (Timeline|Position_Timeline PlayFromStart)
        (else
          (Timeline|Position_Timeline ReverseFromEnd))))))

(event Collision|EventActorBeginOverlap
  (params (OtherActor :type Actor%20Object%20Reference)))

(event EventTick
  (params (DeltaSeconds :type Float%20%28single-precision%29))
  (bind _outactors (Actor|GetAllActorsOfClass 0)))

(fn ConstructionScript)