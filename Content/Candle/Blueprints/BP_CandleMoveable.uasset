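; Physics-simulated candle actor with a Niagara flame, smoke ribbon and optionally randomized mesh, color, scale and rotation.
; While the body is awake, a turbulence timeline turns velocity into fake wind that bends, shrinks and dims flame and wax glow.
; Exceeding BlowOutVelocity can extinguish it, with smoke delayed until the body sleeps.
; Lit and blown-out events take delays for mass use, and probabilistic light spawning limits light count.
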(event OnComponentWake(Candle)
  (params (WakingComponent :type Primitive%20Component%20Object%20Reference) (BoneName :type Name :default "None"))
  ;[1 1 1] Update flame, like wind, but on physics movement
  (CallFunction|PhysicsonFlameMovement))

(event OnComponentSleep(Candle)
  (params (SleepingComponent :type Primitive%20Component%20Object%20Reference) (BoneName :type Name :default "None"))
  ;[1 1 1] Update flame, like wind, but on physics movement
  (CallFunction|StopFlameMovementUpdates)
  (if (Variables|Default|GetBlownOutOnMove)
    (Components|Activation|Activate (Variables|Default|GetSmokeRibbonFX) true)))

(event Custom|BlownOut
  (params (Delay :type Float%20%28single-precision%29))
  ;[1 1 1] Turn candles off
  (Utilities|FlowControl|Delay Delay) ; when blown out enmass add delay so \nthey don't all instantly go out together\nDefault is 0, no delay
  (if (Variables|Default|GetIsLit) ; Test that the candle is indeed lit\nDo nothing if its already unlit
    (CallFunction|CandleUnlit) ; turn off lit params
    (Variables|Default|SetIsLit false)
    (if (not (Class|PrimitiveComponent|IsAnyRigidBodyAwake (Variables|Default|GetCandle))) ; physics is asleep so its safe to trigger smoke
      (Components|Activation|Activate (Variables|Default|GetSmokeRibbonFX) true))))

(event Custom|CandleUnlit
  ;[1 1 1] Turn candles off
  (Rendering|Material|SetScalarParameterValue (Variables|Default|GetCandleMatInst) "IsBurning" 0.0 :!class /Script/Engine.MaterialInstanceDynamic) ; Turn off Flicker and glow
  (Rendering|Material|SetScalarParameterValue (Variables|Default|GetWickMatInst) "IsBurning" 0.0 :!class /Script/Engine.MaterialInstanceDynamic) ; turn off wick glow
  (Components|Activation|Deactivate (Variables|Default|GetFlameParticle)) ; Turn Flame Off
)

(event Custom|StopFlameMovementUpdates
  (bind _flickerscale (Variables|CandleWaxMesh|GetFlickerScale))
  (bind _initialflamesize (Variables|Default|GetInitialFlameSize))
  (bind _lightfalloff (Variables|CandleWaxMesh|GetLightFallOff))
  ;[1 1 1] Update flame, like wind, but on physics movement
  ;;[1 1 1] Set Fade in speed
  (bind (_direction _windturbulencex _windturbulencey _lightscale) (Timeline|MovementWindTurbulence Stop)
    (:Update
      ;;[1 1 1] Get velocity and set it to wind strength
      (bind _returnvalue (Physics|GetPhysicsLinearVelocity (Variables|Default|GetCandle) "None"))
      (bind _outvelocity (CallFunction|RemapVelocity _returnvalue (Variables|Default|GetBlowOutVelocity)))
      (Variables|Wind|SetSpriteAlignDirection (* _outvelocity -1.0)) ; wind direction is opposite of velocity
      (if (<= (Variables|Default|GetBlowOutVelocity) (Math|Vector|VectorLength _returnvalue))
        (if (Variables|Default|GetCanBlowOutFromVelocity)
          (CallFunction|BlownOut 0.0)
          (Variables|Default|SetBlownOutOnMove true) ; tell if smoke should start now or when\nthe candle stops moving
          (else
            (Variables|Wind|SetWind%20Strength (Math|Float|MapRangeClamped (Math|Vector|VectorLength _returnvalue) 0.0 1.2e+03 0.0 1.0) :!label _label)
            ;;[1 1 1] Sprite Alignment/Rotation
            (Class|NiagaraComponent|SetNiagaraVariableVec3 (Variables|Default|GetFlameParticle) "User.SpriteAlignment" (Math|Vector|Normalize (+ (Math|Vector|MakeVector (* _windturbulencex (* (Variables|Wind|GetWind%20Strength) 2.0)) (* (* (Variables|Wind|GetWind%20Strength) 2.0) _windturbulencey) (+ (* (Variables|Wind|GetWind%20Strength) -1.0) 1.0)) (Variables|Wind|GetSpriteAlignDirection)) 0.001)) ; rotate flame away from wind
            ;;[1 1 1] Sprite Scale
            (Class|NiagaraComponent|SetVariableVec2 (Variables|Default|GetFlameParticle) "User.SpriteScale" (Math|Vector2D|MakeVector2D (.x (Math|Vector|Lerp(Vector) (* (Math|Vector|MakeVector (.x _initialflamesize) (.y _initialflamesize) 0.0) (Math|Float|Clamp(Float) (+ (* (Variables|Wind|GetWind%20Strength) -1.0) 1.5))) (Math|Vector|MakeVector 0.3 0.1 0.0) (Math|Float|Clamp(Float) (+ (* (Variables|Wind|GetWind%20Strength) 0.75) (* _lightscale 0.25))))) (.y (Math|Vector|Lerp(Vector) (* (Math|Vector|MakeVector (.x _initialflamesize) (.y _initialflamesize) 0.0) (Math|Float|Clamp(Float) (+ (* (Variables|Wind|GetWind%20Strength) -1.0) 1.5))) (Math|Vector|MakeVector 0.3 0.1 0.0) (Math|Float|Clamp(Float) (+ (* (Variables|Wind|GetWind%20Strength) 0.75) (* _lightscale 0.25))))))) ; scale flame down
            ;;[1 1 1] Material Flicker Speed
            (Niagara|SetNiagaraVariable(Float) (Variables|Default|GetFlameParticle) "User.FlickerSpeed" (Math|Float|Lerp _flickerscale (* _flickerscale 2.0) (Variables|Wind|GetWind%20Strength)))
            ;;[1 1 1] Lighting
            (Effects|Components|ParticleSystem|SetFloatParameter (Variables|Default|GetFlameParticle) "User.LightIntensity" (Math|Float|Lerp 1e+01 0.5 (Variables|Wind|GetWind%20Strength))) ; Dim down Light Intensity on NP_CandleFlameWLight Color Mult
            (Rendering|Material|SetScalarParameterValue (Variables|Default|GetCandleMatInst) "LightFallOff" (Math|Float|Lerp _lightfalloff (* _lightfalloff 0.05) (Math|Float|Clamp(Float) (+ (* (Variables|Wind|GetWind%20Strength) 0.75) (* _lightscale 0.25)))) :!class /Script/Engine.MaterialInstanceDynamic) ; Reduce Light on Wax material when wind blows
          ))
        (else
          (goto _label))))))

(event Custom|CandleLit
  (params (Delay :type Float%20%28single-precision%29))
  (bind _flameparticle (Variables|Default|GetFlameParticle))
  ;[1 1 1] Light Candles
  (Utilities|FlowControl|Delay Delay) ; when get lit enmass add delay so \nthey don't all instantly turn on together\nDefault is 0, no delay
  (Components|Activation|Activate (Variables|Default|GetFlameParticle) true) ; make sure flame is activated, b/c\nits deactivated in blow out
  (if (Variables|Light|GetFlameSpawnParticleLight) ; should particle spawn light?
    (if (>= (Variables|Light|GetLightSpawnPercent) (Math|Random|RandomFloatinRange 0.0 1.0))
      (Niagara|SetNiagaraVariable(Float) _flameparticle "User.LightSpawnProbability" 1.0) ; Optimisation for lighting, to reduce the number \nof lights being spawned, candle either does or \ndoes not spawn light based on %
      (else
        (Niagara|SetNiagaraVariable(Float) _flameparticle "User.LightSpawnProbability" 0.0)))
    (else
      (Niagara|SetNiagaraVariable(Float) (Variables|Default|GetFlameParticle) "User.LightSpawnProbability" 0.0)))
  (Rendering|Material|SetScalarParameterValue (Variables|Default|GetCandleMatInst) "IsBurning" 1.0 :!class /Script/Engine.MaterialInstanceDynamic) ; Turn on Wax Material lighting
  (Rendering|Material|SetScalarParameterValue (Variables|Default|GetWickMatInst) "IsBurning" 1.0 :!class /Script/Engine.MaterialInstanceDynamic) ; Turn on wick material glowing end
  (if (not (Variables|Default|GetIsLit)) ; Checking to see if dynamically lit vs set on start
    (Variables|Default|SetIsLit true)))

(event Custom|PhysicsOnFlameMovement
  (bind _flickerscale (Variables|CandleWaxMesh|GetFlickerScale))
  (bind _initialflamesize (Variables|Default|GetInitialFlameSize))
  (bind _lightfalloff (Variables|CandleWaxMesh|GetLightFallOff))
  ;[1 1 1] Update flame, like wind, but on physics movement
  ;;[1 1 1] Set Fade in speed
  (Components|Timeline|SetNewTime (Variables|Default|GetMovementWindTurbulence) (Math|Random|RandomFloatinRange 0.0 1.0)) ; Offset Loop to avoid uniformity in movement
  (Components|Timeline|SetPlayRate (Variables|Default|GetMovementWindTurbulence) 1.0) ; Set Fade in time, default is 1 second
  (bind (_direction _windturbulencex _windturbulencey _lightscale) (Timeline|MovementWindTurbulence Play)
    (:Update
      ;;[1 1 1] Get velocity and set it to wind strength
      (bind _returnvalue (Physics|GetPhysicsLinearVelocity (Variables|Default|GetCandle) "None"))
      (bind _outvelocity (CallFunction|RemapVelocity _returnvalue (Variables|Default|GetBlowOutVelocity)))
      (Variables|Wind|SetSpriteAlignDirection (* _outvelocity -1.0)) ; wind direction is opposite of velocity
      (if (<= (Variables|Default|GetBlowOutVelocity) (Math|Vector|VectorLength _returnvalue))
        (if (Variables|Default|GetCanBlowOutFromVelocity)
          (CallFunction|BlownOut 0.0)
          (Variables|Default|SetBlownOutOnMove true) ; tell if smoke should start now or when\nthe candle stops moving
          (else
            (Variables|Wind|SetWind%20Strength (Math|Float|MapRangeClamped (Math|Vector|VectorLength _returnvalue) 0.0 1.2e+03 0.0 1.0) :!label _label)
            ;;[1 1 1] Sprite Alignment/Rotation
            (Class|NiagaraComponent|SetNiagaraVariableVec3 (Variables|Default|GetFlameParticle) "User.SpriteAlignment" (Math|Vector|Normalize (+ (Math|Vector|MakeVector (* _windturbulencex (* (Variables|Wind|GetWind%20Strength) 2.0)) (* (* (Variables|Wind|GetWind%20Strength) 2.0) _windturbulencey) (+ (* (Variables|Wind|GetWind%20Strength) -1.0) 1.0)) (Variables|Wind|GetSpriteAlignDirection)) 0.001)) ; rotate flame away from wind
            ;;[1 1 1] Sprite Scale
            (Class|NiagaraComponent|SetVariableVec2 (Variables|Default|GetFlameParticle) "User.SpriteScale" (Math|Vector2D|MakeVector2D (.x (Math|Vector|Lerp(Vector) (* (Math|Vector|MakeVector (.x _initialflamesize) (.y _initialflamesize) 0.0) (Math|Float|Clamp(Float) (+ (* (Variables|Wind|GetWind%20Strength) -1.0) 1.5))) (Math|Vector|MakeVector 0.3 0.1 0.0) (Math|Float|Clamp(Float) (+ (* (Variables|Wind|GetWind%20Strength) 0.75) (* _lightscale 0.25))))) (.y (Math|Vector|Lerp(Vector) (* (Math|Vector|MakeVector (.x _initialflamesize) (.y _initialflamesize) 0.0) (Math|Float|Clamp(Float) (+ (* (Variables|Wind|GetWind%20Strength) -1.0) 1.5))) (Math|Vector|MakeVector 0.3 0.1 0.0) (Math|Float|Clamp(Float) (+ (* (Variables|Wind|GetWind%20Strength) 0.75) (* _lightscale 0.25))))))) ; scale flame down
            ;;[1 1 1] Material Flicker Speed
            (Niagara|SetNiagaraVariable(Float) (Variables|Default|GetFlameParticle) "User.FlickerSpeed" (Math|Float|Lerp _flickerscale (* _flickerscale 2.0) (Variables|Wind|GetWind%20Strength)))
            ;;[1 1 1] Lighting
            (Effects|Components|ParticleSystem|SetFloatParameter (Variables|Default|GetFlameParticle) "User.LightIntensity" (Math|Float|Lerp 1e+01 0.5 (Variables|Wind|GetWind%20Strength))) ; Dim down Light Intensity on NP_CandleFlameWLight Color Mult
            (Rendering|Material|SetScalarParameterValue (Variables|Default|GetCandleMatInst) "LightFallOff" (Math|Float|Lerp _lightfalloff (* _lightfalloff 0.05) (Math|Float|Clamp(Float) (+ (* (Variables|Wind|GetWind%20Strength) 0.75) (* _lightscale 0.25)))) :!class /Script/Engine.MaterialInstanceDynamic) ; Reduce Light on Wax material when wind blows
          ))
        (else
          (goto _label))))))

(event Custom|SetInitialFlameState
  (bind _returnvalue (Math|Random|RandomFloatinRange 0.75 1.2))
  (bind _flameparticle (Variables|Default|GetFlameParticle))
  (bind _globalscale (Variables|CandleWaxMesh|GetGlobalScale))
  (Class|NiagaraComponent|SetNiagaraVariableVec3 (Variables|Default|GetFlameParticle) "User.SpriteAlignment" (Variables|Default|GetCandleFlameAlignment)) ; default candle flame to face "up" in Z
  ;[1 1 1] Random Flame size. Try editing the "Random Uniform Scale Range" to get a wider or more similar flame size. You can also edit the width and height but I found less room for changes there.
  (bind _output_get (Variables|Default|SetInitialFlameSize (Math|Vector2D|MakeVector2D (* (* (Math|Random|RandomFloatinRange 0.9 1.1) _returnvalue) _globalscale) (* _globalscale (* _returnvalue (Math|Random|RandomFloatinRange 0.9 1.15))))))
  (Class|NiagaraComponent|SetVariableVec2 _flameparticle "User.SpriteScale" _output_get) ; Random scale to each candle flame
  (Effects|Components|ParticleSystem|SetFloatParameter _flameparticle "User.LightIntensity" (* (Variables|CandleWaxMesh|GetGlobalScale) 1e+01)) ; Setting the default light brightness on the Niagara \nParticle, I just eye balled it, its not a magic number.
  (Effects|Components|ParticleSystem|SetFloatParameter _flameparticle "User.OffsetFlicker" (Variables|Default|GetRandomCandleID)) ; Random offset to make flames flicker uniquely
  (Effects|Components|ParticleSystem|SetFloatParameter _flameparticle "User.FlickerSpeed" (Variables|CandleWaxMesh|GetFlickerScale)) ; Set the flames distortion flicker scroll speed
  (Effects|Components|ParticleSystem|SetFloatParameter _flameparticle "User.LightRadiusMult" (Variables|CandleWaxMesh|GetGlobalScale)) ; Set the flames distortion flicker scroll speed
  (Effects|Components|ParticleSystem|SetFloatParameter (Variables|Default|GetSmokeRibbonFX) "User.GlobalScale" (Variables|CandleWaxMesh|GetGlobalScale)) ; Set the flames distortion flicker scroll speed
)

(event EventBeginPlay
  (bind _flameparticle (Variables|Default|GetFlameParticle))
  (bind _flameparticle_2 (Variables|Default|GetFlameParticle))
  (bind _candle (Variables|Default|GetCandle))
  ;[1 0 0.5] Begin Play
  (CallFunction|SetInitialFlameState)
  ;[1 1 1] wax and wick material instanced
  (bind _returnvalue (Rendering|Material|CreateDynamicMaterialInstance (Variables|Default|GetCandle) 0 0 "CandleMat" :!class /Script/Engine.PrimitiveComponent))
  (Variables|Default|SetCandleMatInst _returnvalue)
  (bind _returnvalue_2 (Rendering|Material|CreateDynamicMaterialInstance (Variables|Default|GetCandle) 1 0 "CandleWickMat" :!class /Script/Engine.PrimitiveComponent))
  (Variables|Default|SetWickMatInst _returnvalue_2)
  (Rendering|Material|SetScalarParameterValue (Variables|Default|GetCandleMatInst) "OffsetFlicker" (Variables|Default|GetRandomCandleID) :!class /Script/Engine.MaterialInstanceDynamic) ; Wax gets random number for offset in material \nfor fickers so they don't sync
  (if (>= (Variables|Light|GetLightSpawnPercent) (Math|Random|RandomFloatinRange 0.0 1.0))
    (Niagara|SetNiagaraVariable(Float) _flameparticle_2 "User.LightSpawnProbability" 1.0) ; Optimisation for lighting, to reduce the number \nof lights being spawned, candle either does or \ndoes not spawn light based on %
    (else
      (Niagara|SetNiagaraVariable(Float) _flameparticle_2 "User.LightSpawnProbability" 0.0)))
  (Rendering|SetCastShadow (Variables|Default|GetCandle) (Variables|CandleWaxMesh|GetMeshCastShadows)) ; make it easier to manage if the candles \nsticks cast shadows
  (if (Variables|Default|GetIsLit) ; checks that everything is set
    (CallFunction|CandleLit 0.0)
    (else
      (CallFunction|CandleUnlit)))
  ;[1 1 1] Turn Physics ON
  (Physics|SetSimulatePhysics _candle true)
  (Collision|SetCollisionProfileName _candle "PhysicsActor" true :!class /Script/Engine.PrimitiveComponent)
  ;[1 1 1] Its a little easier to calculate scale and rotation when its just one images not a texture sheet.
  (Utilities|FlowControl|MultiGate true false -1
    (:Out%200
      (Effects|Components|ParticleSystem|SetFloatParameter _flameparticle "User.Shape" 0.0) ; Pick Random Flame Shape
    )
    (:Out%201
      (Effects|Components|ParticleSystem|SetFloatParameter _flameparticle "User.Shape" 0.5) ; Pick Random Flame Shape
    )
    (:Out%202
      (Effects|Components|ParticleSystem|SetFloatParameter _flameparticle "User.Shape" 1.0) ; Pick Random Flame Shape
    )))

(fn ConstructionScript
  (bind _globalscale (Variables|CandleWaxMesh|GetGlobalScale))
  (bind _candle (Variables|Default|GetCandle))
  (bind _randomhuefromcolor (Variables|RandomWaxColor|GetRandomHueFromColor))
  (bind _randomsaturation (Variables|RandomWaxColor|GetRandomSaturation))
  (bind _randomvalue (Variables|RandomWaxColor|GetRandomValue))
  (bind _globalscale_2 (Variables|CandleWaxMesh|GetGlobalScale))
  (bind _basecolor (Variables|RandomWaxColor|GetBaseColor))
  (bind _returnvalue (Transformation|GetWorldRotation _candle))
  (bind (_h _s _v) (Math|Color|RGBtoHSV(LinearColor) _basecolor))
  (if (Variables|CandleWaxMesh|GetRandomMesh)
    (Variables|CandleWaxMesh|SetMeshChoice (Utilities|Enum|ByteToEnumE_CandleMeshes (Math|Conversions|ToByte(Integer) (Math|Random|RandomIntegerinRange 0 8)))) ; Pick Random Mesh
  )
  (Components|StaticMesh|SetStaticMesh (Variables|Default|GetCandle) (Utilities|Array|Get(acopy) (LocalVariables|GetCandleMeshes) (Math|Conversions|ToInteger(Byte) (Variables|CandleWaxMesh|GetMeshChoice)))) ; Set Candle Mesh based on choice
  (Transformation|SetRelativeLocation (Variables|Default|GetWickLoc) (Utilities|Array|Get(acopy) (LocalVariables|GetWickLocations) (Math|Conversions|ToInteger(Byte) (Variables|CandleWaxMesh|GetMeshChoice))) false false) ; Set Flame spawn Location to match the candle mesh selected
  ;[1 1 1] Make Material Instances
  (bind _returnvalue_2 (Rendering|Material|CreateDynamicMaterialInstance (Variables|Default|GetCandle) 0 0 "CandleMat" :!class /Script/Engine.PrimitiveComponent)) ; Wax material instance
  (Variables|Default|SetCandleMatInst _returnvalue_2)
  (bind _returnvalue_3 (Rendering|Material|CreateDynamicMaterialInstance (Variables|Default|GetCandle) 1 0 "CandleWickMat" :!class /Script/Engine.PrimitiveComponent)) ; Wick material instance
  (Variables|Default|SetWickMatInst _returnvalue_3)
  (Rendering|Material|SetScalarParameterValue (Variables|Default|GetCandleMatInst) "Saturation" (Variables|CandleWaxMesh|GetLightColorSaturation) :!class /Script/Engine.MaterialInstanceDynamic) ; Since the material forces saturation of the light color for very white candles the light color in the wax can be Desaturated
  (Variables|Default|SetRandomCandleID (Math|Random|RandomFloatinRange 0.0 1e+01)) ; Set Random number used in flicker offset
  (Rendering|Material|SetScalarParameterValue (Variables|Default|GetCandleMatInst) "OffsetFlicker" (Variables|Default|GetRandomCandleID) :!class /Script/Engine.MaterialInstanceDynamic) ; Flicker offset randomly
  (Rendering|Material|SetScalarParameterValue (Variables|Default|GetCandleMatInst) "LightFallOff" (Variables|CandleWaxMesh|GetLightFallOff) :!class /Script/Engine.MaterialInstanceDynamic) ; Certain Colors need less fall off, blues, green, purples
  (Rendering|SetCastShadow (Variables|Default|GetCandle) (Variables|CandleWaxMesh|GetMeshCastShadows)) ; make it easier to set cast shadows
  ;[1 1 1] Rotation
  (if (Variables|CandleWaxMesh|GetRandomRotation)
    (Variables|CandleWaxMesh|SetRotation (Math|Random|RandomFloatinRange -1.8e+02 1.8e+02)) ; Random Rotation Value
    (Transformation|SetWorldRotation _candle (Math|Rotator|MakeRotator (.roll _returnvalue) (.pitch _returnvalue) (Variables|CandleWaxMesh|GetRotation)) false false))
  ;[1 1 1] Scale
  (if (Variables|CandleWaxMesh|GetRandomScale) ; Pick random Mesh? then also random scale
    (Variables|CandleWaxMesh|SetScaleHeight (Math|Random|RandomFloatinRange 0.8 1.2)) ; random height
    (Variables|CandleWaxMesh|SetScaleWidth (Math|Random|RandomFloatinRange 0.8 1.2)) ; random width
    (Transformation|SetRelativeScale3D (Variables|Default|GetCandle) (Math|Vector|MakeVector (* (Variables|CandleWaxMesh|GetScaleWidth) _globalscale) (* (Variables|CandleWaxMesh|GetScaleWidth) _globalscale) (* _globalscale (Variables|CandleWaxMesh|GetScaleHeight)))) ; Set Mesh scales based on user choice
    (else
      (Transformation|SetRelativeScale3D (Variables|Default|GetCandle) (Math|Vector|MakeVector (* (Variables|CandleWaxMesh|GetScaleWidth) _globalscale_2) (* (Variables|CandleWaxMesh|GetScaleWidth) _globalscale_2) (* _globalscale_2 (Variables|CandleWaxMesh|GetScaleHeight)))) ; Manually Set Mesh scale
    ))
  ;[1 1 1] Color
  (if (Variables|RandomWaxColor|GetRandomColor) ; Random Color?
    (bind _output_get (Variables|CandleWaxMesh|SetCandleColor (Class|KismetMathLibrary|HSVtoRGB (+ _h (Math|Random|RandomFloatinRange (* _randomhuefromcolor -1.0) _randomhuefromcolor)) (+ _s (Math|Random|RandomFloatinRange (* _randomsaturation -1.0) _randomsaturation)) (+ _v (Math|Random|RandomFloatinRange (* _randomvalue -1.0) _randomvalue)) 1.0)))
    (Rendering|Material|SetVectorParameterValue (Variables|Default|GetCandleMatInst) "CandleAlbedo" _output_get :!class /Script/Engine.MaterialInstanceDynamic) ; Set Wax Color
    (else
      (Rendering|Material|SetVectorParameterValue (Variables|Default|GetCandleMatInst) "CandleAlbedo" (Variables|CandleWaxMesh|GetCandleColor) :!class /Script/Engine.MaterialInstanceDynamic) ; Set Wax Color
    ))
  ;[1 1 1] Lit
  (if (Variables|Default|GetIsLit) ; Is lit at start? This is also double checked and run at begin play
    (Rendering|Material|SetScalarParameterValue (Variables|Default|GetCandleMatInst) "IsBurning" 1.0 :!class /Script/Engine.MaterialInstanceDynamic)
    (Rendering|Material|SetScalarParameterValue (Variables|Default|GetWickMatInst) "IsBurning" 1.0 :!class /Script/Engine.MaterialInstanceDynamic)
    (else
      (Rendering|Material|SetScalarParameterValue (Variables|Default|GetCandleMatInst) "IsBurning" 0.0 :!class /Script/Engine.MaterialInstanceDynamic)
      (Rendering|Material|SetScalarParameterValue (Variables|Default|GetWickMatInst) "IsBurning" 0.0 :!class /Script/Engine.MaterialInstanceDynamic))))

(fn RemapVelocity
  (params (InVelocity :type Vector) (VelocityMax :type Float%20%28single-precision%29))
  (bind (_x _y _z) (Math|Vector|BreakVector InVelocity))
  (bind _returnvalue (* -1.0 VelocityMax))
  (return (Math|Vector|MakeVector (Math|Float|MapRangeClamped _x _returnvalue VelocityMax -1.0 1.0) (Math|Float|MapRangeClamped _y _returnvalue VelocityMax -1.0 1.0) (Math|Float|MapRangeClamped _z _returnvalue VelocityMax -1.0 1.0))))