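; BP_CandleWind is a spherical wind volume that blows on any BP_Candle overlapping it.
; Overlap begin sends wind strength and the sphere's horizontal forward direction, biased upward to keep flames upright; overlap end triggers the candle's wind fade-out.
; The construction script sets the radius and colors and scales an arrow to preview strength.
; An unconnected timeline can grow the sphere from zero to catch initial overlaps.
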(event OnComponentBeginOverlap(Sphere)
  (params (OverlappedComponent :type Primitive%20Component%20Object%20Reference) (OtherActor :type Actor%20Object%20Reference) (OtherComp :type Primitive%20Component%20Object%20Reference) (OtherBodyIndex :type Integer) (bFromSweep :type Boolean) (SweepResult :type Hit%20Result%20Structure%20%28by%20ref%29))
  (bind _sphere (Variables|Default|GetSphere))
  (bind _returnvalue (Transformation|GetWorldRotation _sphere))
  (bind _returnvalue_2 (Math|Vector|GetForwardVector _returnvalue))
  (bind (_x _y) (Math|Vector|BreakVector _returnvalue_2))
  (bind _asbp_candle (Utilities|Casting|CastToBP_Candle OtherActor)) ; Overlap candle actor?
  (Default|EventWind _asbp_candle (Math|Vector|MakeVector _x _y 0.5) (Variables|Default|GetWindStrength)) ; Trigger wind event on each candle,  Set Candle wind settings
)

(event OnComponentEndOverlap(Sphere)
  (params (OverlappedComponent :type Primitive%20Component%20Object%20Reference) (OtherActor :type Actor%20Object%20Reference) (OtherComp :type Primitive%20Component%20Object%20Reference) (OtherBodyIndex :type Integer))
  (bind _asbp_candle (Utilities|Casting|CastToBP_Candle OtherActor)) ; End overlap candle actor?
  (Default|EventEndWind _asbp_candle) ; Turn wind off (it fades out)
)

(event EventBeginPlay)

(fn ConstructionScript
  (bind _winddirectionalarrow (Variables|Default|GetWindDirectionalArrow))
  ;[1 1 1] Make Arrow Grey if no wind strength set
  (if (> (Variables|Default|GetWindStrength) 0.0)
    (Variables|/Script/Engine.ArrowComponent|SetArrowColor _winddirectionalarrow (LocalVariables|GetUsedColor))
    (else
      (Variables|/Script/Engine.ArrowComponent|SetArrowColor _winddirectionalarrow (LocalVariables|GetUnusedColor))))
  ;[1 1 1] Scale Arrow for visual representation of wind strength
  (Variables|/Script/Engine.ArrowComponent|SetArrowLength (Variables|Default|GetWindDirectionalArrow) (+ (* (Variables|Default|GetWindStrength) 1e+02) 6e+01))
  ;[1 1 1] Sets the... wait for it... the sphere radius!
  (Components|Sphere|SetSphereRadius (Variables|Default|GetSphere) (Variables|Default|GetSphereRadius) false))